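; BP_Owner is a player character that handles world-axis movement, a dash and four attack inputs through a PlayerStatus enum.
; Movement and dash start require the default status, with movement also blocked when dead.
; The dash uses timeline updates to apply a swept forward offset until a counter runs out, then restores the default status.
; Attack inputs only set the status, which Tick prints for debugging.
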(event `InputAxis|MoveForward` :overrideparent false
  (params (AxisValue :type "Float (single-precision)"))
  ;[1 1 1] Move
  (if (`self.CanMove`)
    (`self.AddMovementInput` (1.0 0.0 0.0) AxisValue)))

(event `self.ReceiveBeginPlay`)

(event `InputAxis|MoveRight` :overrideparent false
  (params (AxisValue :type "Float (single-precision)"))
  ;[1 1 1] Move
  (if (`self.CanMove`)
    (`self.AddMovementInput` (0.0 1.0 0.0) AxisValue)))

(event `self.ReceiveTick`
  (params (DeltaSeconds :type "Float (single-precision)"))
  (`KismetSystemLibrary.PrintString` (`|GetEnumeratorNameAsString` (`self.PlayerStatus`))))

(event `InputAction|Dash`
  (params (Key :type "Key Structure"))
  (:`Pressed`
    (if (`self.CanDash`)
      (set `self.DashCounter` 20)
      (set `self.PlayerStatus` "NewEnumerator6")
      (`self.DashStart`))))

(event `InputAction|PointAttack`
  (params (Key :type "Key Structure"))
  (:`Pressed`
    (set `self.PlayerStatus` "NewEnumerator1")))

(event `InputAction|LengeAttack`
  (params (Key :type "Key Structure"))
  (:`Pressed`
    (set `self.PlayerStatus` "NewEnumerator3")))

(event `DashStart`
  (`Timeline|DashLine` :!via `PlayFromStart` :!label _label
    (:`Update`
      (`self.DashTick`))))

(event `InputAction|UniqueAttack`
  (params (Key :type "Key Structure"))
  (:`Pressed`
    (set `self.PlayerStatus` "NewEnumerator4")))

(event `DashEnd`
  (goto _label :!via `Stop`))

(event `InputAction|SpecialAttack`
  (params (Key :type "Key Structure"))
  (:`Pressed`
    (set `self.PlayerStatus` "NewEnumerator5")))

(fn `CanDash`
  (returns (ReturnValue :type Boolean))
  (if (and (`|EnumEquality` (`self.PlayerStatus`) "NewEnumerator0") (== (`self.DashCounter`) 0))
    (return true)
    (else
      (return false))))

(fn `CanMove`
  (returns (ReturnValue :type Boolean))
  (locals (isDead :type Boolean))
  (if (and (not (`local.isDead`)) (`|EnumEquality` (`self.PlayerStatus`) "NewEnumerator0"))
    (return true)
    (else
      (return false))))

(fn `DashTick`
  (locals (DashSpeed :type "Float (double-precision)" :default 20.0))
  (if (> (`self.DashCounter`) 0)
    (`self.K2_AddActorLocalOffset` (`KismetMathLibrary.MakeVector` (`local.DashSpeed`)) true)
    (`/Engine/EditorBlueprintResources/StandardMacros.DecrementInt` (`self.DashCounter`))
    (elif (`|EnumEquality` (`self.PlayerStatus`) "NewEnumerator6")
      (set `self.PlayerStatus` "NewEnumerator0")
      (`self.DashEnd`))))

(fn `UserConstructionScript`)