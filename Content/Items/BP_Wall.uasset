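; BP_Wall is a networked wall that gets knocked a fixed step along its local X axis when a BP_Bullet overlaps its Cube.
; The overlap passes the bullet's velocity to HitRunOnServer, which picks the push direction from the sign of its X component.
; On authority, a Tick timer periodically sends the Cube's world location through ForceSyncMulticast, which teleports the Cube to correct drift.
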(event `self.ReceiveTick`
  (params (DeltaSeconds :type "Float (single-precision)"))
  (`/Engine/EditorBlueprintResources/ActorMacros.Switch Has Authority`
    (:`Authority`
      (bind _output_get (set `self.Timer` (+ DeltaSeconds (`self.Timer`))))
      (if (>= _output_get (`self.LimitTimer`))
        (set `self.Timer` 0.0)
        (`self.ForceSyncMulticast` (`SceneComponent.K2_GetComponentLocation` (`self.Cube`)))))))

(event `ForceSyncMulticast`
  (params (NewLocation :type "Vector Structure"))
  ;[1 1 1] 強制同期
  (`SceneComponent.K2_SetWorldLocation` (`self.Cube`) NewLocation false true))

(event `self.Cube.OnComponentBeginOverlap`
  (params (OverlappedComponent :type "PrimitiveComponent Object Reference") (OtherActor :type "Actor Object Reference") (OtherComp :type "PrimitiveComponent Object Reference") (OtherBodyIndex :type Integer) (bFromSweep :type Boolean) (SweepResult :type "HitResult Structure (by ref)"))
  ;[1 1 1] Hit判定
  (bind _asbp_bullet (cast `/Game/Character/Mannequin/BP_Bullet` OtherActor))
  (`self.HitRunOnServer` _asbp_bullet (`self.GetVelocity` _asbp_bullet)))

(event `HitRunOnServer`
  (params (`ターゲット` :type "Actor Object Reference") (DeltaLocation :type "Vector Structure"))
  ;[1 1 1] Hit判定
  (`self.K2_AddActorLocalOffset` (`KismetMathLibrary.SelectVector` (50.0 0.0 0.0) (-50.0 0.0 0.0) (>= (.x DeltaLocation) 0.0))))

(fn `UserConstructionScript`)