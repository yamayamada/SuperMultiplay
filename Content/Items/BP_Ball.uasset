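; BP_Ball is a ball item actor that periodically forces its position to stay in sync across the network.
; On Tick, only the authority accumulates a timer and, each time it reaches LimitTimer, resets it and passes the Sphere's world location to ForceSyncMulticast.
; That event teleports the Sphere to the received location without sweeping, a hard correction with no interpolation.
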(event `self.ReceiveTick`
  (params (DeltaSeconds :type "Float (single-precision)"))
  (`/Engine/EditorBlueprintResources/ActorMacros.Switch Has Authority`
    (:`Authority`
      (bind _output_get (set `self.Timer` (+ DeltaSeconds (`self.Timer`))))
      (if (>= _output_get (`self.LimitTimer`))
        (set `self.Timer` 0.0)
        (`self.ForceSyncMulticast` (`SceneComponent.K2_GetComponentLocation` (`self.Sphere`)))))))

(event `ForceSyncMulticast`
  (params (NewLocation :type "Vector Structure"))
  ;[1 1 1] 強制同期
  (`SceneComponent.K2_SetWorldLocation` (`self.Sphere`) NewLocation false true))

(fn `UserConstructionScript`)